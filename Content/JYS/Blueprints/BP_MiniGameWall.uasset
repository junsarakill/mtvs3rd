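; BP_MiniGameWall is a wall actor, named for a minigame, that fades in or out through two custom events.
; SetFadein and SetFadeOut each play a timeline that drives the Opacity parameter on a dynamic material instance, created on every update from the Cube's material.
; Fade-out also disables the Cube's collision, which fade-in does not restore.
; Both fades play the same 2D sound when finished.
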(event `self.ReceiveBeginPlay`)

(event `self.SetFadeIn`
  (bind _cube (`self.Cube`))
  (bind (_direction _opacity) (`Timeline|FadeIn`)
    (:`Update`
      (bind _returnvalue (`PrimitiveComponent.CreateDynamicMaterialInstance` _cube 0 (`PrimitiveComponent.GetMaterial` _cube 0) "None"))
      (`MaterialInstanceDynamic.SetScalarParameterValue` _returnvalue "Opacity" _opacity))
    (:`Finished`
      (`GameplayStatics.PlaySound2D` "/Game/JYS/Blueprints/elegant-commercial-logo-for-video-production-153322.elegant-commercial-logo-for-video-production-153322" 1.0 1.0 0.0 null null))))

(event `self.SetFadeOut`
  (bind _cube (`self.Cube`))
  (bind (_direction _opacity) (`Timeline|FadeOut`)
    (:`Update`
      (bind _returnvalue (`PrimitiveComponent.CreateDynamicMaterialInstance` _cube 0 (`PrimitiveComponent.GetMaterial` _cube 0) "None"))
      (`MaterialInstanceDynamic.SetScalarParameterValue` _returnvalue "Opacity" _opacity)
      (`PrimitiveComponent.SetCollisionEnabled` (`self.Cube`) "NoCollision"))
    (:`Finished`
      (`GameplayStatics.PlaySound2D` "/Game/JYS/Blueprints/elegant-commercial-logo-for-video-production-153322.elegant-commercial-logo-for-video-production-153322" 1.0 1.0 0.0 null null))))

(fn `UserConstructionScript`)