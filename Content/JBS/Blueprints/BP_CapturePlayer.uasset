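; BP_CapturePlayer is a capture actor that renders a character skeletal mesh in isolation through a SceneCaptureComponent2D.
; On BeginPlay the scene capture is set to show only the SkeletalMesh component.
; SetMesh looks up a type in MeshMap and applies that entry's mesh and animation class to the component, printing the mesh names to screen.
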(event `self.ReceiveBeginPlay`
  (`SceneCaptureComponent.ShowOnlyComponent` (`self.SceneCaptureComponent2D`) (`self.SkeletalMesh`)))

(event `self.SetMesh`
  (params (type :type "EPlayerType Enum" :default "MALE1"))
  (bind _skeletalmesh (`self.SkeletalMesh`))
  (bind (_value _returnvalue) (`BlueprintMapLibrary.Map_Find` (`self.meshMap`) type))
  (if _returnvalue
    (`KismetSystemLibrary.PrintString` (`KismetSystemLibrary.GetDisplayName` (`.mesh` (break `CapturePlayer` _value))))
    (`SkeletalMeshComponent.SetSkeletalMeshAsset` _skeletalmesh (`.mesh` (break `CapturePlayer` _value)))
    (`SkeletalMeshComponent.SetAnimInstanceClass` _skeletalmesh (`.anim` (break `CapturePlayer` _value)))
    (`KismetSystemLibrary.PrintString` (`KismetSystemLibrary.GetDisplayName` (`SkeletalMeshComponent.GetSkeletalMeshAsset` _skeletalmesh)))))

(fn `UserConstructionScript`)