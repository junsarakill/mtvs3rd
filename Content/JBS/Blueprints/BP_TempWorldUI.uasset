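; BP_TempWorldUI is a world-space UI actor that keeps its Widget component turned toward the player's camera.
; BeginPlay caches the camera manager of player controller 0.
; Each Tick, if that manager is valid, it billboards the widget by setting its world rotation along the direction from the widget to the camera location.
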(event `self.ReceiveBeginPlay`
  (set `self.Player Camera Manager` (`PlayerController.PlayerCameraManager` (`GameplayStatics.GetPlayerController` 0))))

(event `self.ReceiveTick`
  (params (DeltaSeconds :type "Float (single-precision)"))
  (bind _widget (`self.Widget`))
  (bind _player_camera_manager (`self.Player Camera Manager`)
    (:`then`
      (`SceneComponent.K2_SetWorldRotation` _widget (`KismetMathLibrary.Conv_VectorToRotator` (- (`PlayerCameraManager.GetCameraLocation` _player_camera_manager) (`SceneComponent.K2_GetComponentLocation` _widget))) false false))
    (:`else`)))

(fn `UserConstructionScript`)