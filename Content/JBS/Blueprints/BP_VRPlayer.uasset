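; BP_VRPlayer is the VR player pawn, which sets stage tracking, offsets its root to a set camera height and adds input mapping contexts.
; It spawns left and right BP_Hand actors attached to the VR root.
; Enhanced Input events drive turning and movement, and forward grab and trigger presses to each hand, with triggers also toggling its ray.
; Finger inputs write pose alphas into each hand's ABP_MannequinsXR animation instance.
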(event `self.ReceiveBeginPlay`
  (bind (_returnvalue_x _returnvalue_y _returnvalue_z) (`KismetMathLibrary.BreakVector` (`SceneComponent.K2_GetComponentLocation` (`self.vrHMDCam`))))
  (`|ExecutionSequence`
    (:`then_0`
      (`HeadMountedDisplayFunctionLibrary.SetTrackingOrigin` "Stage")
      (`SceneComponent.K2_AddRelativeLocation` (`self.vrRoot`) (`KismetMathLibrary.MakeVector` 0.0 0.0 (- (`self.cameraHeight`) _returnvalue_z)) false false))
    (:`then_1`
      (`self.SpawnLRController`))
    (:`then_2`
      (`self.SetIMC` "/Game/JBS/Input/IMC_BS_Default.IMC_BS_Default")
      (`self.SetIMC` "/Game/JBS/Input/IMC_BS_Hand.IMC_BS_Hand"))))

(event `self.ReceiveTick`
  (params (DeltaSeconds :type "Float (single-precision)")))

(event `EnhancedInput|/Game/VRTemplate/Input/Actions/IA_Turn`
  (params (ActionValue :type "Float (double-precision)") (ElapsedSeconds :type "Float (double-precision)") (TriggeredSeconds :type "Float (double-precision)") (InputAction :type "InputAction Object Reference" :default "/Game/VRTemplate/Input/Actions/IA_Turn.IA_Turn"))
  (:`Started`
    (`self.EventTurn` ActionValue)))

(event `EnhancedInput|/Game/JBS/Input/IA_BS_Move`
  (params (ActionValue :type "Vector2D Structure") (ElapsedSeconds :type "Float (double-precision)") (TriggeredSeconds :type "Float (double-precision)") (InputAction :type "InputAction Object Reference" :default "/Game/JBS/Input/IA_BS_Move.IA_BS_Move"))
  (:`Triggered`
    (`self.SetMoveDir` ActionValue :!label _label))
  (:`Started`
    (goto _label))
  (:`Canceled`
    (goto _label))
  (:`Completed`
    (goto _label)))

(event `EnhancedInput|/Game/VRTemplate/Input/Actions/IA_Grab_Right`
  (params (ActionValue :type "Float (double-precision)") (ElapsedSeconds :type "Float (double-precision)") (TriggeredSeconds :type "Float (double-precision)") (InputAction :type "InputAction Object Reference" :default "/Game/VRTemplate/Input/Actions/IA_Grab_Right.IA_Grab_Right"))
  (bind _rightcontroller (`self.rightController`))
  (:`Started`
    (`BS_Hand.TryGrab` _rightcontroller))
  (:`Completed`
    (`BS_Hand.TryRelease` _rightcontroller)))

(event `EnhancedInput|/Game/VRTemplate/Input/Actions/IA_Grab_Left`
  (params (ActionValue :type "Float (double-precision)") (ElapsedSeconds :type "Float (double-precision)") (TriggeredSeconds :type "Float (double-precision)") (InputAction :type "InputAction Object Reference" :default "/Game/VRTemplate/Input/Actions/IA_Grab_Left.IA_Grab_Left"))
  (bind _leftcontroller (`self.leftController`))
  (:`Started`
    (`BS_Hand.TryGrab` _leftcontroller))
  (:`Completed`
    (`BS_Hand.TryRelease` _leftcontroller)))

(event `EnhancedInput|/Game/JBS/Input/IA_BS_Trigger_Left`
  (params (ActionValue :type Boolean) (ElapsedSeconds :type "Float (double-precision)") (TriggeredSeconds :type "Float (double-precision)") (InputAction :type "InputAction Object Reference" :default "/Game/JBS/Input/IA_BS_Trigger_Left.IA_BS_Trigger_Left"))
  (:`Started`
    (bind _leftcontroller (`self.leftController`)
      (:`then`
        (`BS_Hand.EventPressLMB` _leftcontroller)
        (`BS_Hand.SetEnableRay` _leftcontroller true))
      (:`else`)))
  (:`Completed`
    (bind _leftcontroller_2 (`self.leftController`)
      (:`then`
        (`BS_Hand.EventReleaseLMB` _leftcontroller_2)
        (`BS_Hand.SetEnableRay` _leftcontroller_2 false))
      (:`else`))))

(event `EnhancedInput|/Game/JBS/Input/IA_BS_Trigger_Right`
  (params (ActionValue :type Boolean) (ElapsedSeconds :type "Float (double-precision)") (TriggeredSeconds :type "Float (double-precision)") (InputAction :type "InputAction Object Reference" :default "/Game/JBS/Input/IA_BS_Trigger_Right.IA_BS_Trigger_Right"))
  (:`Started`
    (bind _rightcontroller (`self.rightController`)
      (:`then`
        (`BS_Hand.EventPressLMB` _rightcontroller)
        (`BS_Hand.SetEnableRay` _rightcontroller true))
      (:`else`)))
  (:`Completed`
    (bind _rightcontroller_2 (`self.rightController`)
      (:`then`
        (`BS_Hand.EventReleaseLMB` _rightcontroller_2)
        (`BS_Hand.SetEnableRay` _rightcontroller_2 false))
      (:`else`))))

(event `EnhancedInput|/Game/VRTemplate/Input/Actions/Hands/IA_Hand_Grasp_Right`
  (params (ActionValue :type "Float (double-precision)") (ElapsedSeconds :type "Float (double-precision)") (TriggeredSeconds :type "Float (double-precision)") (InputAction :type "InputAction Object Reference" :default "/Game/VRTemplate/Input/Actions/Hands/IA_Hand_Grasp_Right.IA_Hand_Grasp_Right"))
  (bind _rightcontroller (`self.rightController`))
  ;[1 1 1] hand input
  (:`Triggered`
    (`self.HandGrasp` _rightcontroller ActionValue))
  (:`Canceled`
    (`self.HandGrasp` _rightcontroller :!label _label_2))
  (:`Completed`
    (goto _label_2)))

(event `EnhancedInput|/Game/VRTemplate/Input/Actions/Hands/IA_Hand_Grasp_Left`
  (params (ActionValue :type "Float (double-precision)") (ElapsedSeconds :type "Float (double-precision)") (TriggeredSeconds :type "Float (double-precision)") (InputAction :type "InputAction Object Reference" :default "/Game/VRTemplate/Input/Actions/Hands/IA_Hand_Grasp_Left.IA_Hand_Grasp_Left"))
  (bind _leftcontroller (`self.leftController`))
  ;[1 1 1] hand input
  (:`Triggered`
    (`self.HandGrasp` _leftcontroller ActionValue))
  (:`Canceled`
    (`self.HandGrasp` _leftcontroller :!label _label_3))
  (:`Completed`
    (goto _label_3)))

(event `EnhancedInput|/Game/VRTemplate/Input/Actions/Hands/IA_Hand_Point_Left`
  (params (ActionValue :type "Float (double-precision)") (ElapsedSeconds :type "Float (double-precision)") (TriggeredSeconds :type "Float (double-precision)") (InputAction :type "InputAction Object Reference" :default "/Game/VRTemplate/Input/Actions/Hands/IA_Hand_Point_Left.IA_Hand_Point_Left"))
  (bind _leftcontroller (`self.leftController`))
  ;[1 1 1] hand input
  (:`Started`
    (`self.HandPoint` _leftcontroller :!label _label_4))
  (:`Canceled`
    (goto _label_4))
  (:`Completed`
    (`self.HandPoint` _leftcontroller 1.0)))

(event `EnhancedInput|/Game/VRTemplate/Input/Actions/Hands/IA_Hand_Point_Right`
  (params (ActionValue :type "Float (double-precision)") (ElapsedSeconds :type "Float (double-precision)") (TriggeredSeconds :type "Float (double-precision)") (InputAction :type "InputAction Object Reference" :default "/Game/VRTemplate/Input/Actions/Hands/IA_Hand_Point_Right.IA_Hand_Point_Right"))
  (bind _rightcontroller (`self.rightController`))
  ;[1 1 1] hand input
  (:`Started`
    (`self.HandPoint` _rightcontroller :!label _label_5))
  (:`Canceled`
    (goto _label_5))
  (:`Completed`
    (`self.HandPoint` _rightcontroller 1.0)))

(event `EnhancedInput|/Game/VRTemplate/Input/Actions/Hands/IA_Hand_IndexCurl_Left`
  (params (ActionValue :type "Float (double-precision)") (ElapsedSeconds :type "Float (double-precision)") (TriggeredSeconds :type "Float (double-precision)") (InputAction :type "InputAction Object Reference" :default "/Game/VRTemplate/Input/Actions/Hands/IA_Hand_IndexCurl_Left.IA_Hand_IndexCurl_Left"))
  (bind _leftcontroller (`self.leftController`))
  ;[1 1 1] hand input
  (:`Triggered`
    (`BS_Hand.handMesh` _leftcontroller
      (:`then`
        (bind _returnvalue (`SkeletalMeshComponent.GetAnimInstance` (stale _handmesh)))
        (bind _asabp_mannequins_xr (cast `/Game/Characters/MannequinsXR/Meshes/ABP_MannequinsXR` _returnvalue))
        (set `/Game/Characters/MannequinsXR/Meshes/ABP_MannequinsXR.PoseAlphaIndexCurl` ActionValue _asabp_mannequins_xr))
      (:`else`)))
  (:`Canceled`
    (bind _handmesh (`BS_Hand.handMesh` _leftcontroller :!label _label_6)
      (:`then`
        (bind _asabp_mannequins_xr_2 (cast `/Game/Characters/MannequinsXR/Meshes/ABP_MannequinsXR` _returnvalue))
        (set `/Game/Characters/MannequinsXR/Meshes/ABP_MannequinsXR.PoseAlphaIndexCurl` 0.0 _asabp_mannequins_xr_2))
      (:`else`)))
  (:`Completed`
    (goto _label_6)))

(event `EnhancedInput|/Game/VRTemplate/Input/Actions/Hands/IA_Hand_IndexCurl_Right`
  (params (ActionValue :type "Float (double-precision)") (ElapsedSeconds :type "Float (double-precision)") (TriggeredSeconds :type "Float (double-precision)") (InputAction :type "InputAction Object Reference" :default "/Game/VRTemplate/Input/Actions/Hands/IA_Hand_IndexCurl_Right.IA_Hand_IndexCurl_Right"))
  (bind _rightcontroller (`self.rightController`))
  ;[1 1 1] hand input
  (:`Triggered`
    (bind _handmesh (`BS_Hand.handMesh` _rightcontroller)
      (:`then`
        (bind _returnvalue (`SkeletalMeshComponent.GetAnimInstance` _handmesh))
        (bind _asabp_mannequins_xr (cast `/Game/Characters/MannequinsXR/Meshes/ABP_MannequinsXR` _returnvalue))
        (set `/Game/Characters/MannequinsXR/Meshes/ABP_MannequinsXR.PoseAlphaIndexCurl` ActionValue _asabp_mannequins_xr))
      (:`else`)))
  (:`Canceled`
    (`BS_Hand.handMesh` _rightcontroller :!label _label_7
      (:`then`
        (bind _asabp_mannequins_xr_2 (cast `/Game/Characters/MannequinsXR/Meshes/ABP_MannequinsXR` _returnvalue))
        (set `/Game/Characters/MannequinsXR/Meshes/ABP_MannequinsXR.PoseAlphaIndexCurl` 0.0 _asabp_mannequins_xr_2))
      (:`else`)))
  (:`Completed`
    (goto _label_7)))

(event `EnhancedInput|/Game/VRTemplate/Input/Actions/Hands/IA_Hand_ThumbUp_Left`
  (params (ActionValue :type "Float (double-precision)") (ElapsedSeconds :type "Float (double-precision)") (TriggeredSeconds :type "Float (double-precision)") (InputAction :type "InputAction Object Reference" :default "/Game/VRTemplate/Input/Actions/Hands/IA_Hand_ThumbUp_Left.IA_Hand_ThumbUp_Left"))
  (bind _leftcontroller (`self.leftController`))
  ;[1 1 1] hand input
  (:`Started`
    (bind _handmesh (`BS_Hand.handMesh` _leftcontroller :!label _label_8)
      (:`then`
        (bind _asabp_mannequins_xr (cast `/Game/Characters/MannequinsXR/Meshes/ABP_MannequinsXR` (`SkeletalMeshComponent.GetAnimInstance` _handmesh)))
        (set `/Game/Characters/MannequinsXR/Meshes/ABP_MannequinsXR.PoseAlphaThumbUp` 0.0 _asabp_mannequins_xr))
      (:`else`)))
  (:`Canceled`
    (goto _label_8))
  (:`Completed`
    (bind _handmesh_2 (`BS_Hand.handMesh` _leftcontroller)
      (:`then`
        (bind _asabp_mannequins_xr_2 (cast `/Game/Characters/MannequinsXR/Meshes/ABP_MannequinsXR` (`SkeletalMeshComponent.GetAnimInstance` _handmesh_2)))
        (set `/Game/Characters/MannequinsXR/Meshes/ABP_MannequinsXR.PoseAlphaThumbUp` 1.0 _asabp_mannequins_xr_2))
      (:`else`))))

(event `EnhancedInput|/Game/VRTemplate/Input/Actions/Hands/IA_Hand_ThumbUp_Right`
  (params (ActionValue :type "Float (double-precision)") (ElapsedSeconds :type "Float (double-precision)") (TriggeredSeconds :type "Float (double-precision)") (InputAction :type "InputAction Object Reference" :default "/Game/VRTemplate/Input/Actions/Hands/IA_Hand_ThumbUp_Right.IA_Hand_ThumbUp_Right"))
  (bind _rightcontroller (`self.rightController`))
  ;[1 1 1] hand input
  (:`Started`
    (bind _handmesh (`BS_Hand.handMesh` _rightcontroller :!label _label_9)
      (:`then`
        (bind _asabp_mannequins_xr (cast `/Game/Characters/MannequinsXR/Meshes/ABP_MannequinsXR` (`SkeletalMeshComponent.GetAnimInstance` _handmesh)))
        (set `/Game/Characters/MannequinsXR/Meshes/ABP_MannequinsXR.PoseAlphaThumbUp` 0.0 _asabp_mannequins_xr))
      (:`else`)))
  (:`Canceled`
    (goto _label_9))
  (:`Completed`
    (bind _handmesh_2 (`BS_Hand.handMesh` _rightcontroller)
      (:`then`
        (bind _asabp_mannequins_xr_2 (cast `/Game/Characters/MannequinsXR/Meshes/ABP_MannequinsXR` (`SkeletalMeshComponent.GetAnimInstance` _handmesh_2)))
        (set `/Game/Characters/MannequinsXR/Meshes/ABP_MannequinsXR.PoseAlphaThumbUp` 1.0 _asabp_mannequins_xr_2))
      (:`else`))))

(fn `HandGrasp`
  (params (hand :type "BS_Hand Object Reference") (alpha :type "Float (double-precision)"))
  (bind _handmesh (`BS_Hand.handMesh` hand)
    (:`then`
      (bind _asabp_mannequins_xr (cast `/Game/Characters/MannequinsXR/Meshes/ABP_MannequinsXR` (`SkeletalMeshComponent.GetAnimInstance` _handmesh)))
      (set `/Game/Characters/MannequinsXR/Meshes/ABP_MannequinsXR.PoseAlphaGrasp` alpha _asabp_mannequins_xr))
    (:`else`)))

(fn `HandPoint`
  (params (hand :type "BS_Hand Object Reference") (alpha :type "Float (double-precision)"))
  (bind _handmesh (`BS_Hand.handMesh` hand)
    (:`then`
      (bind _asabp_mannequins_xr (cast `/Game/Characters/MannequinsXR/Meshes/ABP_MannequinsXR` (`SkeletalMeshComponent.GetAnimInstance` _handmesh)))
      (set `/Game/Characters/MannequinsXR/Meshes/ABP_MannequinsXR.PoseAlphaPoint` alpha _asabp_mannequins_xr))
    (:`else`)))

(fn `SpawnLRController`
  (bind _vrroot (`self.vrRoot`))
  (`|ExecutionSequence`
    (:`then_0`
      (bind _returnvalue (`|SpawnActorFromClass` "/Game/JBS/Blueprints/BP_Hand.BP_Hand_C" (`KismetMathLibrary.MakeTransform` (0.0 0.0 0.0)) "Undefined" "MultiplyWithRoot" self null))
      (bind _output_get (set `self.leftController` _returnvalue))
      (`BS_Hand.SetController` _output_get "LEFT")
      (`self.K2_AttachToComponent` _output_get _vrroot "None" "SnapToTarget" "SnapToTarget" "SnapToTarget" true))
    (:`then_1`
      (bind _returnvalue_2 (`|SpawnActorFromClass` "/Game/JBS/Blueprints/BP_Hand.BP_Hand_C" (`KismetMathLibrary.MakeTransform` (0.0 0.0 0.0)) "Undefined" "MultiplyWithRoot" self null))
      (bind _output_get_2 (set `self.rightController` _returnvalue_2))
      (`BS_Hand.SetController` _output_get_2 "RIGHT")
      (`self.K2_AttachToComponent` _output_get_2 _vrroot "None" "SnapToTarget" "SnapToTarget" "SnapToTarget" true))))

(fn `UserConstructionScript`)